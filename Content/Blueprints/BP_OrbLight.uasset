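; BP_OrbLight is an orb with a point light that shows one of four orb states: none, Fire, Electric or Plasma.
; UpdateOrbLight stores the new state, swaps the orb mesh material, and either zeroes the light for No Orb or calls SetLightAttributes.
; SetLightAttributes applies a large radius, high intensity and a color matching the state.
; The event graph and construction script are empty, so changes happen only when UpdateOrbLight is called.
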(event EventBeginPlay)

(event Collision|EventActorBeginOverlap
  (params (OtherActor :type Actor%20Object%20Reference)))

(event EventTick
  (params (DeltaSeconds :type Float%20%28single-precision%29)))

(fn ConstructionScript)

(fn SetLightAttributes
  (bind _pointlight (Variables|Default|GetPointLight))
  (Rendering|Lighting|SetAttenuationRadius _pointlight 1.5e+04)
  (Rendering|Components|Light|SetIntensity _pointlight 5e+04)
  (switch Utilities|FlowControl|Switch|SwitchonEOrbType (Variables|Default|GetOrbColor)
    (:OT_None
      (Rendering|Components|Light|SetLightColor :self _pointlight))
    (:OT_Fire
      (Rendering|Components|Light|SetLightColor _pointlight "(R=0.906250,G=0.000000,B=0.000000,A=1.000000)" true))
    (:OT_Electric
      (Rendering|Components|Light|SetLightColor _pointlight "(R=0.088542,G=0.423622,B=1.000000,A=1.000000)" true))
    (:OT_Plasma
      (Rendering|Components|Light|SetLightColor _pointlight "(R=1.000000,G=0.000000,B=0.889065,A=1.000000)" true))))

(fn UpdateOrbLight
  (params (NewOrbColor :type EOrbType%20Enum :default "OT_None"))
  (bind _orbmesh (Variables|Default|GetOrbMesh))
  (bind _defaultsceneroot (Variables|Default|GetDefaultSceneRoot))
  (bind _pointlight (Variables|Default|GetPointLight))
  (bind _output_get (Variables|Default|SetOrbColor NewOrbColor))
  (switch Utilities|FlowControl|Switch|SwitchonEOrbType _output_get
    (:OT_None
      (Rendering|Material|SetMaterial _orbmesh 0 "/Game/Dev/Materials/M_Orb_Base.M_Orb_Base")
      (Development|SetHiddeninGame _defaultsceneroot false false)
      (Class|LightComponent|SetLightFunctionDisabledBrightness _pointlight 0.0)
      (Rendering|Lighting|SetAttenuationRadius _pointlight 0.0)
      (Rendering|Components|Light|SetIntensity _pointlight 0.0))
    (:OT_Fire
      (Rendering|Material|SetMaterial _orbmesh 0 "/Game/Dev/Materials/MI_Orb_Fire.MI_Orb_Fire")
      (Development|SetHiddeninGame _defaultsceneroot false false :!label _label)
      (Class|LightComponent|SetLightFunctionDisabledBrightness _pointlight 1.0)
      (CallFunction|SetLightAttributes))
    (:OT_Electric
      (Rendering|Material|SetMaterial _orbmesh 0 "/Game/Dev/Materials/MI_Orb_Shock.MI_Orb_Shock")
      (goto _label))
    (:OT_Plasma
      (Rendering|Material|SetMaterial _orbmesh 0 "/Game/Dev/Materials/MI_Orb_Plasma.MI_Orb_Plasma")
      (goto _label))))