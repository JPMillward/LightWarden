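; Fire island platform that crumbles when overlapped while active, then reappears.
; On begin play it binds to the Light Warden game mode's new world state event, marking WardenPlatform active only when the world orb matches its platform orb.
; An overlap while active waits TimeToCrumble, hides the actor and disables its collision, then restores both after a fixed delay.
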(event Custom|OnNewWorldState
  (params (OrbState :type EOrbType%20Enum%20%28by%20ref%29 :default "OT_None"))
  (CallFunction|UpdateFirePlatform OrbState))

(event EventBeginPlay
  (|CallParentFunction)
  (bind _asbp_light_warden_game_mode (Utilities|Casting|CastToBP_LightWardenGameMode (Game|GetGameMode)))
  (EventDispatchers|BindEventtoNewWorldState _asbp_light_warden_game_mode (delegate Custom|OnNewWorldState)))

(event Collision|EventActorBeginOverlap
  (params (OtherActor :type Actor%20Object%20Reference))
  (if (Variables|/Script/LightWarden.WardenPlatformComponent|GetIsPlatformActive (Variables|Default|GetWardenPlatform))
    (Utilities|FlowControl|Delay (Variables|Default|GetTimeToCrumble))
    (Collision|SetActorEnableCollision false)
    (Rendering|SetActorHiddenInGame true)
    (Utilities|FlowControl|Delay 5.0)
    (Collision|SetActorEnableCollision true)
    (Rendering|SetActorHiddenInGame false)))

(event EventTick
  (params (DeltaSeconds :type Float%20%28single-precision%29))
  (|CallParentFunction DeltaSeconds) ; This node is disabled and will not be called.\nDrag off pins to build functionality.
)

(fn ConstructionScript
  (|CallParentFunction))

(fn UpdateFirePlatform
  (params (WorldOrb :type EOrbType%20Enum%20%28by%20ref%29 :default "OT_None"))
  (bind _wardenplatform (Variables|Default|GetWardenPlatform))
  (Variables|/Script/LightWarden.WardenPlatformComponent|SetIsPlatformActive _wardenplatform (Utilities|Enum|Equal(Enum) WorldOrb (Variables|/Script/LightWarden.WardenPlatformComponent|GetPlatformOrb _wardenplatform))))