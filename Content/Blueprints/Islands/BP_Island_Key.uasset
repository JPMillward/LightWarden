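; BP_Island_Key is an island puzzle actor that toggles a lock platform based on the orb held by its pedestal.
; The construction script caches the BP_Island_Lock child actor.
; BeginPlay checks the child BP_Pedestal's current orb and binds the same check to orb swaps.
; A DoNotTouch orb hides the lock and disables its collision, while any other value shows it and restores collision.
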(event Custom|CheckPlatformLock
  (params (PedestalOrb :type EOrbType%20Enum%20%28by%20ref%29 :default "OT_None"))
  (bind _as_bp_island_lock (Variables|Default|GetAs%20BP%20Island%20Lock))
  (if (Utilities|Enum|Equal(Enum) PedestalOrb (Variables|Default|Getdo%20not%20touch))
    (Rendering|SetActorHiddenInGame _as_bp_island_lock true)
    (Collision|SetActorEnableCollision _as_bp_island_lock false)
    (else
      (Rendering|SetActorHiddenInGame _as_bp_island_lock false)
      (Collision|SetActorEnableCollision _as_bp_island_lock true))))

(event EventBeginPlay
  (|CallParentFunction)
  (bind _asbp_pedestal (Utilities|Casting|CastToBP_Pedestal (Variables|/Script/Engine.ChildActorComponent|GetChildActor (Variables|Default|GetPedestalChild%20Actor)))
    (:then
      (CallFunction|CheckPlatformLock (Variables|/Script/LightWarden.OrbPedestal|GetPedestalOrb _asbp_pedestal))
      (EventDispatchers|BindEventtoOrbSwap _asbp_pedestal (delegate Custom|CheckPlatformLock)))
    (:CastFailed
      (Development|PrintString "cast failed"))))

(event Collision|EventActorBeginOverlap
  (params (OtherActor :type Actor%20Object%20Reference))
  (|CallParentFunction OtherActor) ; This node is disabled and will not be called.\nDrag off pins to build functionality.
)

(event EventTick
  (params (DeltaSeconds :type Float%20%28single-precision%29))
  (|CallParentFunction DeltaSeconds) ; This node is disabled and will not be called.\nDrag off pins to build functionality.
)

(fn ConstructionScript
  (|CallParentFunction)
  (bind _asbp_island_lock (Utilities|Casting|CastToBP_Island_Lock (Variables|/Script/Engine.ChildActorComponent|GetChildActor (Variables|Components|GetLock%20Platform))))
  (Variables|Default|SetAs%20BP%20Island%20Lock _asbp_island_lock))