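; BP_Island_Plasma is a plasma island platform that appears or disappears with the world's orb state.
; It binds to the LightWarden game mode's world-state event and marks itself active when the new orb matches its WardenPlatform's PlatformOrb.
; Active platforms are visible with collision; inactive ones are hidden without it.
; Both BeginPlay branches hide the platform, so it only appears after a matching state update.
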(event Custom|OnPlatformUpdate
  (params (OrbState :type EOrbType%20Enum%20%28by%20ref%29 :default "OT_None"))
  (CallFunction|UpdatePlasmaPlatform OrbState))

(event EventBeginPlay
  (|CallParentFunction)
  (bind _asbp_light_warden_game_mode (Utilities|Casting|CastToBP_LightWardenGameMode (Game|GetGameMode)))
  (EventDispatchers|BindEventtoNewWorldState _asbp_light_warden_game_mode (delegate Custom|OnPlatformUpdate))
  (if (Variables|/Script/LightWarden.WardenPlatformComponent|GetIsPlatformActive (Variables|Default|GetWardenPlatform))
    (Collision|SetActorEnableCollision false)
    (Rendering|SetActorHiddenInGame true)
    (else
      (Collision|SetActorEnableCollision false)
      (Rendering|SetActorHiddenInGame true))))

(event Collision|EventActorBeginOverlap
  (params (OtherActor :type Actor%20Object%20Reference))
  (|CallParentFunction OtherActor) ; This node is disabled and will not be called.\nDrag off pins to build functionality.
)

(event EventTick
  (params (DeltaSeconds :type Float%20%28single-precision%29))
  (|CallParentFunction DeltaSeconds) ; This node is disabled and will not be called.\nDrag off pins to build functionality.
)

(fn ConstructionScript
  (|CallParentFunction))

(fn UpdatePlasmaPlatform
  (params (WorldOrb :type EOrbType%20Enum%20%28by%20ref%29 :default "OT_None"))
  (bind _wardenplatform (Variables|Default|GetWardenPlatform))
  (bind _output_get (Variables|/Script/LightWarden.WardenPlatformComponent|SetIsPlatformActive _wardenplatform (Utilities|Enum|Equal(Enum) WorldOrb (Variables|/Script/LightWarden.WardenPlatformComponent|GetPlatformOrb _wardenplatform))))
  (if _output_get
    (Development|PrintString "PlasmaPlatform Update  TRUE")
    (Collision|SetActorEnableCollision true)
    (Rendering|SetActorHiddenInGame false)
    (else
      (Development|PrintString "PlasmaPlatform False")
      (Collision|SetActorEnableCollision false)
      (Rendering|SetActorHiddenInGame true))))