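; Electric moving-platform island that travels only while an actor overlaps it and the world's orb state matches the platform's orb.
; It listens to the LightWarden game mode's world-state event to set the active flag, which is checked when an overlap begins.
; A timeline lerps it to a scaled end offset, with a hold delay and FlipFlop alternating direction.
; Ending overlap stops the timeline, and re-entry resumes in the last direction.
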(event Custom|OnNewWorldState
  (params (OrbState :type EOrbType%20Enum%20%28by%20ref%29 :default "OT_None"))
  ;[1 1 1] Begin Play
  (CallFunction|UpdateElectricPlatform OrbState))

(event Custom|ForwardMovement
  (bind _wardenplatform (Variables|Default|GetWardenPlatform))
  (bind _platformtransform (Variables|/Script/LightWarden.WardenPlatformComponent|GetPlatformTransform _wardenplatform))
  ;[1 1 1] Platform Movement Timer
  (Development|PrintString "forward movement called")
  (Variables|Default|SetbIsForward true)
  (if (Variables|Default|GetIsStopped)
    (Development|PrintString "Intercvepted Movement Call")
    (else
      (bind (_direction _alpha) (Timeline|PlatformMovementAnim Play)
        (:Update
          (bind _output_get (Variables|Default|SetLerpAlpha _alpha))
          (switch Utilities|FlowControl|Switch|SwitchonETimelineDirection _direction
            (:Forward
              _)
            (:Backward
              _))
          (Transformation|SetActorRelativeLocation (Math|Vector|Lerp(Vector) (.location _platformtransform) (+ (.location _platformtransform) (* (.scale _platformtransform) (Variables|Default|GetEnd%20Destination))) _output_get)))
        (:Finished
          (Utilities|FlowControl|Delay (Variables|Default|GetHoldTime))
          (Utilities|FlowControl|FlipFlop
            (:A
              (CallFunction|ReverseMovement))
            (:B
              (CallFunction|ForwardMovement))))))))

(event Custom|ReverseMovement
  (bind _wardenplatform (Variables|Default|GetWardenPlatform))
  (bind _platformtransform (Variables|/Script/LightWarden.WardenPlatformComponent|GetPlatformTransform _wardenplatform))
  ;[1 1 1] Platform Movement Timer
  (Development|PrintString "reverse movement called")
  (Variables|Default|SetbIsForward false)
  (if (Variables|Default|GetIsStopped)
    (Development|PrintString "Intercvepted Movement Call")
    (else
      (bind (_direction _alpha) (Timeline|PlatformMovementAnim Reverse)
        (:Update
          (bind _output_get (Variables|Default|SetLerpAlpha _alpha))
          (switch Utilities|FlowControl|Switch|SwitchonETimelineDirection _direction
            (:Forward
              _)
            (:Backward
              _))
          (Transformation|SetActorRelativeLocation (Math|Vector|Lerp(Vector) (.location _platformtransform) (+ (.location _platformtransform) (* (.scale _platformtransform) (Variables|Default|GetEnd%20Destination))) _output_get)))
        (:Finished
          (Utilities|FlowControl|Delay (Variables|Default|GetHoldTime))
          (Utilities|FlowControl|FlipFlop
            (:A
              (CallFunction|ReverseMovement))
            (:B
              (CallFunction|ForwardMovement))))))))

(event Custom|StopMoving
  (bind _wardenplatform (Variables|Default|GetWardenPlatform))
  (bind _platformtransform (Variables|/Script/LightWarden.WardenPlatformComponent|GetPlatformTransform _wardenplatform))
  ;[1 1 1] Platform Movement Timer
  (Development|PrintString "stop moving called")
  (bind (_direction _alpha) (Timeline|PlatformMovementAnim Stop)
    (:Update
      (bind _output_get (Variables|Default|SetLerpAlpha _alpha))
      (switch Utilities|FlowControl|Switch|SwitchonETimelineDirection _direction
        (:Forward
          _)
        (:Backward
          _))
      (Transformation|SetActorRelativeLocation (Math|Vector|Lerp(Vector) (.location _platformtransform) (+ (.location _platformtransform) (* (.scale _platformtransform) (Variables|Default|GetEnd%20Destination))) _output_get)))
    (:Finished
      (Utilities|FlowControl|Delay (Variables|Default|GetHoldTime))
      (Utilities|FlowControl|FlipFlop
        (:A
          (CallFunction|ReverseMovement))
        (:B
          (CallFunction|ForwardMovement))))))

(event Custom|BeginMoving
  ;[1 1 1] Platform Movement Timer
  (Development|PrintString "beginmoving")
  (if (Variables|Default|GetbIsForward)
    (CallFunction|ForwardMovement)
    (else
      (CallFunction|ReverseMovement))))

(event EventBeginPlay
  ;[1 1 1] Begin Play
  (|CallParentFunction)
  (bind _asbp_light_warden_game_mode (Utilities|Casting|CastToBP_LightWardenGameMode (Game|GetGameMode)))
  (EventDispatchers|BindEventtoNewWorldState _asbp_light_warden_game_mode (delegate Custom|OnNewWorldState)))

(event Collision|EventActorBeginOverlap
  (params (OtherActor :type Actor%20Object%20Reference))
  ;[1 1 1] Player Overlap
  (if (Variables|/Script/LightWarden.WardenPlatformComponent|GetIsPlatformActive (Variables|Default|GetWardenPlatform))
    (bind _output_get (Variables|Default|SetIsStopped false))
    (Development|PrintString (Utilities|String|ToString(Boolean) _output_get))
    (CallFunction|BeginMoving)))

(event EventTick
  (params (DeltaSeconds :type Float%20%28single-precision%29))
  (|CallParentFunction DeltaSeconds) ; This node is disabled and will not be called.\nDrag off pins to build functionality.
)

(event Collision|EventActorEndOverlap
  (params (OtherActor :type Actor%20Object%20Reference))
  ;[1 1 1] Player Overlap
  (Variables|Default|SetIsStopped true)
  (CallFunction|StopMoving))

(fn ConstructionScript
  (|CallParentFunction))

(fn UpdateElectricPlatform
  (params (WorldOrb :type EOrbType%20Enum%20%28by%20ref%29 :default "OT_None"))
  (bind _wardenplatform (Variables|Default|GetWardenPlatform))
  (bind _platformorb (Variables|/Script/LightWarden.WardenPlatformComponent|GetPlatformOrb _wardenplatform))
  (Development|PrintString (Utilities|String|Append "World Orb Is:" (Utilities|String|EnumtoString WorldOrb)))
  (Development|PrintString (Utilities|String|Append "Platform Orb Is:" (Utilities|String|EnumtoString _platformorb)))
  (bind _output_get (Variables|/Script/LightWarden.WardenPlatformComponent|SetIsPlatformActive _wardenplatform (Utilities|Enum|Equal(Enum) WorldOrb _platformorb)))
  (if _output_get
    (Development|PrintString "Electricplatform Update  TRUE")
    (else
      (Development|PrintString "ElectricPlatform False"))))