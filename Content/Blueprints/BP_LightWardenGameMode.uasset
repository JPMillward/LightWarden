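; Game mode for Light Warden that respawns the player character at a checkpoint and broadcasts orb-driven world state changes.
; On begin play it records the player's transform as the checkpoint and binds to the character's destroyed event.
; On death it spawns and possesses a new character at the checkpoint, rebinds that event, signals a reset and restores the saved orb.
; Orb swaps pass the saved orb to the new-world-state call.
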(event Custom|OnOrbSwap
  (CallFunction|SetActiveOrbState))

(event Custom|RespawnPlayer
  (params (DestroyedActor :type Actor%20Object%20Reference))
  (CallFunction|HandlePlayerRespawn))

(event Custom|Respawn
  (bind _asbp_light_warden_character (Utilities|Casting|CastToBP_LightWardenCharacter (Game|GetPlayerCharacter 0)))
  (Game|AssignOnDestroyed _asbp_light_warden_character (delegate Custom|RespawnPlayer)))

(event EventBeginPlay
  (Utilities|FlowControl|Sequence
    (:then_0
      (bind _asbp_light_warden_character (Utilities|Casting|CastToBP_LightWardenCharacter (Game|GetPlayerCharacter 0)))
      (Game|AssignOnDestroyed _asbp_light_warden_character (delegate Custom|RespawnPlayer)))
    (:then_1
      (Class|LightWardenGameMode|SetCheckPoint (Transformation|GetActorTransform (Game|GetPlayerCharacter 0))))))

(event EventTick
  (params (DeltaSeconds :type Float%20%28single-precision%29)))

(fn ConstructionScript)

(fn SetActiveOrbState
  (bind _returnvalue (Class|LightWardenGameMode|GetSavedOrb))
  (Default|CallNewWorldState _returnvalue))

(fn HandlePlayerRespawn
  (bind _returnvalue (Class|LightWardenGameMode|GetCheckPoint))
  (bind _returnvalue_2 (Game|SpawnActorfromClass "/Game/Blueprints/BP_LightWardenCharacter.BP_LightWardenCharacter_C" _returnvalue "Undefined" 0 0))
  (Pawn|Possess (Game|GetPlayerController 0) _returnvalue_2)
  (CallFunction|Respawn)
  (Class|LightWardenGameMode|OnPlayerReset _returnvalue_2)
  (bind _returnvalue_3 (Class|LightWardenGameMode|GetSavedOrb))
  (Class|LightWardenCharacter|SetPlayerOrb _returnvalue_2 _returnvalue_3)
  (Default|UpdateOrbSocket _returnvalue_2))