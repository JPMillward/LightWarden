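; BP_Pedestal is an interactable orb holder that passes orbs to and from the Light Warden player character.
; Interacting sets the checkpoint at player zero's transform, then picks a transfer from player and pedestal orb states, with debug prints as placeholder negative feedback.
; Transfers update the child BP_OrbLight and player socket, then report holder, saved orb and swap to the game mode.
; The construction script also refreshes the child orb.
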(event EventBeginPlay)

(event Collision|EventActorBeginOverlap
  (params (OtherActor :type Actor%20Object%20Reference)))

(event EventTick
  (params (DeltaSeconds :type Float%20%28single-precision%29)))

(event EventStartFocus
  (Development|PrintString "Interactive Object Found"))

(event EventEndFocus
  (Development|PrintString "Lost Interactive Object"))

(event EventOnInteract
  (params (InteractCaller :type Actor%20Object%20Reference))
  (bind _pedestalorb (Variables|Default|GetPedestalOrb))
  (Utilities|FlowControl|Sequence
    (:then_0
      ;[1 1 1] Set Player Respawn Point
      (Development|PrintString "On Interact Called")
      (bind _aslight_warden_game_mode (Utilities|Casting|CastToLightWardenGameMode (Game|GetGameMode)))
      (Class|LightWardenGameMode|SetCheckPoint _aslight_warden_game_mode (Transformation|GetActorTransform (Game|GetPlayerCharacter 0))))
    (:then_1
      (bind _asbp_light_warden_character (Utilities|Casting|CastToBP_LightWardenCharacter InteractCaller))
      (bind _returnvalue (Class|LightWardenCharacter|DoesHaveOrb _asbp_light_warden_character))
      (if _returnvalue :!label _label
        (CallFunction|PassOrbtoPedestal _asbp_light_warden_character (Variables|/Script/LightWarden.LightWardenCharacter|GetPlayerOrbSlot _asbp_light_warden_character))
        (else
          (Development|PrintString "Neither Has Orb,Give Negative Feedback"))))
    (:then_2
      (if (Utilities|Enum|Equal(Enum) "OT_None" _pedestalorb)
        (goto _label)
        (elif _returnvalue
          (Development|PrintString "Both Have Orb, Give Negative Feedback")
          (else
            (CallFunction|PassOrbtoPlayer _pedestalorb _asbp_light_warden_character)))))))

(fn ConstructionScript
  (CallFunction|UpdateChildOrb))

(fn PassOrbtoPedestal
  (params (Player :type BP%20Light%20Warden%20Character%20Object%20Reference) (OrbType :type EOrbType%20Enum :default "OT_None"))
  (bind _output_get (Variables|Default|SetPedestalOrb OrbType))
  (bind _output_get_2 (Variables|/Script/LightWarden.LightWardenCharacter|SetPlayerOrbSlot Player "OT_None"))
  (CallFunction|UpdateChildOrb)
  (Default|UpdateOrbSocket Player)
  (bind _asbp_light_warden_game_mode (Utilities|Casting|CastToBP_LightWardenGameMode (Game|GetGameMode)))
  (Class|LightWardenGameMode|UpdateOrbHolder _asbp_light_warden_game_mode _output_get self)
  (Class|LightWardenGameMode|SetSavedOrb _asbp_light_warden_game_mode _output_get_2)
  (Default|OnOrbSwap _asbp_light_warden_game_mode)
  (Default|CallOrbSwap _output_get))

(fn PassOrbtoPlayer
  (params (PedestalOrbType :type EOrbType%20Enum :default "OT_None") (PlayerCharacter :type BP%20Light%20Warden%20Character%20Object%20Reference))
  (bind _output_get (Variables|/Script/LightWarden.LightWardenCharacter|SetPlayerOrbSlot PlayerCharacter PedestalOrbType))
  (bind _output_get_2 (Variables|Default|SetPedestalOrb "OT_None"))
  (CallFunction|UpdateChildOrb)
  (Default|UpdateOrbSocket PlayerCharacter)
  (bind _asbp_light_warden_game_mode (Utilities|Casting|CastToBP_LightWardenGameMode (Game|GetGameMode)))
  (Class|LightWardenGameMode|UpdateOrbHolder _asbp_light_warden_game_mode _output_get PlayerCharacter)
  (Class|LightWardenGameMode|SetSavedOrb _asbp_light_warden_game_mode _output_get)
  (Default|OnOrbSwap _asbp_light_warden_game_mode)
  (Default|CallOrbSwap _output_get_2))

(fn UpdateChildOrb
  (bind _returnvalue (Class|OrbPedestal|GetOrbType))
  (bind _asbp_orb_light (Utilities|Casting|CastToBP_OrbLight (Variables|/Script/Engine.ChildActorComponent|GetChildActor (Variables|Default|GetOrbLight)))
    (:then
      (Default|UpdateOrbLight _asbp_orb_light _returnvalue))
    (:CastFailed
      (Development|PrintString "cast fail?"))))